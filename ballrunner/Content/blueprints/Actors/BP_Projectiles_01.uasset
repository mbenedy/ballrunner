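; BP_Projectiles_01 is a projectile actor that restarts the current level when it hits the player.
; Its Sphere component's hit event compares against player pawn 0, reopens the current level by name on a match, and destroys the actor on any hit.
; Tick feeds a Delay set by the Deleteproject variable into DestroyActor, acting as a lifetime timer.
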(event OnComponentHit(Sphere)
  (params (HitComponent :type Primitive%20Component%20Object%20Reference) (OtherActor :type Actor%20Object%20Reference) (OtherComp :type Primitive%20Component%20Object%20Reference) (NormalImpulse :type Vector :default "0, 0, 0") (Hit :type Hit%20Result%20Structure%20%28by%20ref%29))
  (if (== 0 (Game|Player|GetPlayerPawn 0))
    (bind _returnvalue (Game|GetCurrentLevelName true))
    (Game|OpenLevel(byName) (Utilities|String|StringToName _returnvalue))
    (Actor|DestroyActor)
    (else
      (Actor|DestroyActor))))

(event EventTick
  (params (DeltaSeconds :type Float%20%28single-precision%29))
  (Utilities|FlowControl|Delay (Variables|Default|Getdeleteproject))
  (Actor|DestroyActor))

(fn ConstructionScript)