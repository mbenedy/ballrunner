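; BP_Cannon_01 is a cannon actor that automatically fires BP_Projectiles_01 on a repeating cycle.
; After a start delay, it waits for FireRate, then spawns a scaled projectile at its Arrow component's world location and rotation.
; The CannonShoot timeline animates recoil along the Cannon component's relative Y and restarts the wait on finishing, so the shot interval includes the recoil time.
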(event EventBeginPlay
  (bind _arrow (Variables|Default|Getarrow))
  (Utilities|FlowControl|Delay (Variables|Default|Getdelaystart))
  (Utilities|FlowControl|Delay (Variables|Shooting|GetFireRate) :!label _label)
  (Game|SpawnActorfromClass "/Game/blueprints/Actors/BP_Projectiles_01.BP_Projectiles_01_C" (Math|Transform|MakeTransform (Transformation|GetWorldLocation _arrow) (Transformation|GetWorldRotation _arrow) (Variables|Default|GetProjectileScale)) "Undefined" 0 0)
  (bind _cannonrecoil (Timeline|CannonShoot PlayFromStart)
    (:Update
      (Transformation|SetRelativeLocation (Variables|Default|GetCannon) (Math|Vector|MakeVector 0.0 _cannonrecoil 0.0) false false))
    (:Finished
      (goto _label))))

(fn ConstructionScript)